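; BP_Knight is the player knight character, with single-axis movement, jumping, a three-step sword combo, blocking, parry and shield bash.
; Inputs set state flags that gate actions, drive Animator montages and set walk speed.
; Blocking raises the shield after a timer delay, turning Parry into a shield bash; Parry currently ignores its CanAttack check.
; Sword and shield hitbox overlaps damage BP_Dummy, then disable both hitboxes.
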(event OnComponentBeginOverlap(ShieldHitbox)
  (params (OverlappedComponent :type Primitive%20Component%20Object%20Reference) (OtherActor :type Actor%20Object%20Reference) (OtherComp :type Primitive%20Component%20Object%20Reference) (OtherBodyIndex :type Integer) (bFromSweep :type Boolean) (SweepResult :type Hit%20Result%20Structure%20%28by%20ref%29))
  ;[1 1 1] Hitreg
  (bind _asbp_dummy (Utilities|Casting|CastToBP_Dummy OtherActor))
  (Default|TakeDamage _asbp_dummy)
  (CallFunction|DisableAttackHitboxes))

(event OnComponentBeginOverlap(SwordHitbox)
  (params (OverlappedComponent :type Primitive%20Component%20Object%20Reference) (OtherActor :type Actor%20Object%20Reference) (OtherComp :type Primitive%20Component%20Object%20Reference) (OtherBodyIndex :type Integer) (bFromSweep :type Boolean) (SweepResult :type Hit%20Result%20Structure%20%28by%20ref%29))
  ;[1 1 1] Hitreg
  (bind _asbp_dummy (Utilities|Casting|CastToBP_Dummy OtherActor))
  (Default|TakeDamage _asbp_dummy)
  (CallFunction|DisableAttackHitboxes))

(event Custom|ShieldUpTImer
  (CallFunction|OnShieldUp))

(event EventBeginPlay
  ;[1 1 1] Locomotion
  (CallFunction|InitPlayer))

(event Input|ActionEvents|InputActionParry
  (params (Key :type Key%20Structure :default "None"))
  (:Pressed
    (Variables|Default|SetParryKeyPressed true)
    (CallFunction|CanAttack)
    (if true
      (if (Variables|Default|GethasShieldUp)
        (CallFunction|SetShieldBashAttack)
        (else
          (CallFunction|SetParryAttack)))))
  (:Released
    (Variables|Default|SetParryKeyPressed false)))

(event Input|ActionEvents|InputActionBlock
  (params (Key :type Key%20Structure :default "None"))
  (:Pressed
    (Variables|Default|SetBlockKeyPressed true)
    (CallFunction|SetBlocking true))
  (:Released
    (Variables|Default|SetBlockKeyPressed false)
    (CallFunction|SetBlocking false)))

(event Input|ActionEvents|InputActionAttack
  (params (Key :type Key%20Structure :default "None"))
  (:Pressed
    (bind _value (CallFunction|CanAttack))
    (if _value
      (CallFunction|CheckAddtoCombo)
      (CallFunction|ExecuteCurrentCombo)
      (Variables|Default|SetcomboInputAllowed false)
      (CallFunction|SetAttacking true))))

(event Input|ActionEvents|InputActionJump
  (params (Key :type Key%20Structure :default "None"))
  ;[1 1 1] Locomotion
  (:Pressed
    (Character|Jump))
  (:Released
    (Character|StopJumping)))

(event Input|AxisEvents|InputAxisMoveRight
  (params (AxisValue :type Float%20%28single-precision%29))
  ;[1 1 1] Locomotion
  (bind _value (CallFunction|CanMove))
  (if _value
    (Pawn|Input|AddMovementInput "0,-1.000000, 0" AxisValue false)))

(fn ConstructionScript)

(fn InitPlayer
  (CallFunction|SetMovementSpeed)
  (CallFunction|SetCharacterMovementSpeed)
  (CallFunction|DisableAttackHitboxes))

(fn SetAnimator
  (params (Animator :type ABP%20Knight%20Object%20Reference))
  (Variables|Default|SetAnimator Animator))

(fn SetComboInputAllowed
  (params (value :type Boolean))
  (bind _output_get (Variables|Default|SetcomboInputAllowed value))
  (if _output_get
    _))

(fn CanMove
  (return (not (Math|Boolean|ORBoolean (Variables|Default|GetisAttacking) (Variables|Default|GetisStunned) (Variables|Default|GetisFlinching) (Variables|Default|GetisDeath)))))

(fn CanAttack
  (return (and (not (Math|Boolean|ANDBoolean (Variables|Default|GetisDeath) (Variables|Default|GetisStunned) (Variables|Default|GetisFlinching))) (Variables|Default|GetcomboInputAllowed))))

(fn CanBlock
  (return (not (Math|Boolean|ORBoolean (Variables|Default|GetisAttacking) (Variables|Default|GetisStunned) (Variables|Default|GetisFlinching) (Variables|Default|GetisDeath)))))

(fn CheckAddtoCombo
  (if (and (Variables|Default|GetcomboInputAllowed) (Math|Integer|InRange(Integer) (Variables|Default|GetCurrentCombo) 0 2))
    (bind _result (Math|Integer|IncrementInt (Variables|Default|GetCurrentCombo))
      (:%20%20
        (Variables|Default|SetCurrentCombo _result)))))

(fn ExecuteCurrentCombo
  (if (Math|Integer|InRange(Integer) (Variables|Default|GetCurrentCombo) 1 3)
    (Variables|Default|SetcomboInputAllowed false)
    (Animation|Montage|MontagePlay (Variables|Default|GetAnimator) (Variables|Default|GetComboMontage) 0.7 "MontageLength" 0.0 true)
    (Ability|Animation|MontageJumptoSection (Variables|Default|GetAnimator) (Utilities|String|StringToName (Utilities|String|ToString(Integer) (Variables|Default|GetCurrentCombo))) (Variables|Default|GetComboMontage))
    (else
      (return))))

(fn SetJumpingAttack
  (params (Jumping :type Boolean))
  (if Jumping
    (Pawn|Components|CharacterMovement|SetMovementMode (Variables|Character|GetCharacterMovement) "MOVE_Flying" 0)
    (else
      (Pawn|Components|CharacterMovement|SetMovementMode (Variables|Character|GetCharacterMovement) "MOVE_Walking" 0))))

(fn SetMovementSpeed
  (if (Variables|Default|GetisBlocking)
    (Variables|Default|SetcurrentMovementSpeed (Variables|Default|GetwalkingSpeed))
    (elif (Variables|Default|GetisSprinting)
      (Variables|Default|SetcurrentMovementSpeed (Variables|Default|GetsprintingSpeed))
      (else
        (Variables|Default|SetcurrentMovementSpeed (Variables|Default|GetrunningSpeed)))))
  (return))

(fn SetCharacterMovementSpeed
  (Variables|/Script/Engine.CharacterMovementComponent|SetMaxWalkSpeed (Variables|Character|GetCharacterMovement) (Variables|Default|GetcurrentMovementSpeed)))

(fn ChangeStateSwordHitbox
  (params (enabled :type Boolean))
  (Variables|/Script/Engine.PrimitiveComponent|SetbGenerateOverlapEvents (Variables|Default|GetSwordHitbox) enabled))

(fn ChangeStateShieldHitbox
  (params (enabled :type Boolean))
  (Variables|/Script/Engine.PrimitiveComponent|SetbGenerateOverlapEvents (Variables|Default|GetShieldHitbox) enabled))

(fn DisableAttackHitboxes
  (CallFunction|ChangeStateSwordHitbox false)
  (CallFunction|ChangeStateShieldHitbox false))

(fn GetMovementSpeed
  (return (Math|Float|Absolute(Float) (.y (Variables|/Script/Engine.MovementComponent|GetVelocity (Variables|Character|GetCharacterMovement))))))

(fn SetBlocking
  (params (value :type Boolean))
  (bind _output_get (Variables|Default|SetisBlocking value))
  (Utilities|FlowControl|Sequence
    (:then_0
      (if _output_get
        (bind _canblock (CallFunction|CanBlock))
        (if _canblock
          (if (not (Animation|Montage|MontageIsPlaying (Variables|Default|GetAnimator) (Variables|Default|GetBlockMontage)))
            (Animation|Montage|MontagePlay (Variables|Default|GetAnimator) (Variables|Default|GetBlockMontage) 1.0 "MontageLength" 0.0 true)
            (bind _returnvalue (Utilities|Time|SetTimerbyFunctionName 0 "ShieldUpTImer" (Variables|Default|GetShieldUpDelay)))
            (Variables|Default|SetShieldUpTimerEvent _returnvalue))
          (else
            (Variables|Default|SetisBlocking false)
            (CallFunction|OnShieldDown)))
        (else
          (Animation|Montage|MontageStop (Variables|Default|GetAnimator) 0.25 (Variables|Default|GetBlockMontage))
          (CallFunction|OnShieldDown))))
    (:then_1
      (CallFunction|SetMovementSpeed)
      (CallFunction|SetCharacterMovementSpeed))))

(fn SetAttacking
  (params (Value :type Boolean))
  (bind _output_get (Variables|Default|SetisAttacking Value))
  (Default|SetAttacking (Variables|Default|GetAnimator) _output_get "NewEnumerator0")
  (if _output_get
    (Variables|Default|SetnewComboQueued true)
    (Variables|Default|SetcomboInputAllowed false)
    (CallFunction|SetBlocking false)
    (else
      (Variables|Default|SetcomboInputAllowed true)
      (Variables|Default|SetnewComboQueued false)
      (Variables|Default|SetCurrentCombo 0)
      (Animation|Montage|MontageStop (Variables|Default|GetAnimator) 0.1 (Variables|Default|GetComboMontage)))))

(fn SetParryAttack
  (bind _output_get (Variables|Default|SetisAttacking true))
  (Default|SetAttacking (Variables|Default|GetAnimator) _output_get "NewEnumerator1")
  (if _output_get
    (Variables|Default|SetnewComboQueued true)
    (Variables|Default|SetcomboInputAllowed false)
    (CallFunction|SetBlocking false)
    (Variables|Default|SetCurrentCombo 0)
    (else
      (Variables|Default|SetcomboInputAllowed true)
      (Variables|Default|SetnewComboQueued false)
      (Variables|Default|SetCurrentCombo 0))))

(fn SetShieldBashAttack
  (bind _output_get (Variables|Default|SetisAttacking true))
  (Default|SetAttacking (Variables|Default|GetAnimator) _output_get "NewEnumerator2")
  (if _output_get
    (Variables|Default|SetnewComboQueued true)
    (Variables|Default|SetcomboInputAllowed false)
    (CallFunction|SetBlocking false)
    (Variables|Default|SetCurrentCombo 0)
    (else
      (Variables|Default|SetcomboInputAllowed true)
      (Variables|Default|SetnewComboQueued false)
      (Variables|Default|SetCurrentCombo 0))))

(fn OnShieldUp
  (Variables|Default|SethasShieldUp true)
  (Development|PrintString "rikisima la papita" true true "(R=1.000000,G=0.953554,B=0.020501,A=1.000000)"))

(fn OnShieldDown
  (Variables|Default|SethasShieldUp false)
  (Utilities|Time|ClearandInvalidateTimerbyHandle (Variables|Default|GetShieldUpTimerEvent)))