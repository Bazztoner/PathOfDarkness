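; Dragonaut boss Blueprint that plays a sword-whip attack as a chain of Paper2D flipbook animations.
; AttackStart plays the anticipation flipbook, whose finished event triggers AttackEnableHitbox to spawn BP_Dummy and play the active swing.
; When the swing finishes, OnAttackEnd spawns BP_DamageDummy and restores the looping walk, with both spawns at the boss's transform.
; Nothing here calls AttackStart, and SetAnimation is an empty stub.
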(event Custom|AttackStart
  (bind _bosssprites (Variables|Default|GetBossSprites))
  (Sprite|SetFlipbook _bosssprites "/Game/PathOfDarkness/Characters/Bosses/Dragonaut/Animations/SwordWhip/1_Anticipation/Dragonaut_SwordWhipe_Anticipation.Dragonaut_SwordWhipe_Anticipation")
  (Components|Timeline|PlayfromStart _bosssprites)
  (Components|Timeline|SetLooping _bosssprites false)
  (EventDispatchers|BindEventtoOnFinishedPlaying _bosssprites (delegate Custom|AttackEnableHitbox)))

(event Custom|AttackEnableHitbox
  (bind _bosssprites (Variables|Default|GetBossSprites))
  (EventDispatchers|UnbindallEventsfromOnFinishedPlaying _bosssprites)
  (Game|SpawnActorfromClass "/Game/Dummy/BP_Dummy.BP_Dummy_C" (Transformation|GetActorTransform) "Undefined" 0 0)
  (Sprite|SetFlipbook _bosssprites "/Game/PathOfDarkness/Characters/Bosses/Dragonaut/Animations/SwordWhip/2_Active/Dragonaut_SwordWhip_Active.Dragonaut_SwordWhip_Active")
  (Components|Timeline|PlayfromStart _bosssprites)
  (Components|Timeline|SetLooping (Variables|Default|GetBossSprites) false)
  (EventDispatchers|AssignOnFinishedPlaying _bosssprites (delegate Custom|OnAttackEnd)))

(event Custom|OnAttackEnd
  (bind _bosssprites (Variables|Default|GetBossSprites))
  (EventDispatchers|UnbindallEventsfromOnFinishedPlaying _bosssprites)
  (Game|SpawnActorfromClass "/Game/PathOfDarkness/Dummys/BP_DamageDummy.BP_DamageDummy_C" (Transformation|GetActorTransform) "Undefined" 0 0)
  (Sprite|SetFlipbook _bosssprites "/Game/PathOfDarkness/Characters/Bosses/Dragonaut/Animations/Walk/Dragonaut_Walk.Dragonaut_Walk")
  (Components|Timeline|PlayfromStart _bosssprites)
  (Components|Timeline|SetLooping _bosssprites true))

(event EventBeginPlay)

(fn ConstructionScript)

(fn SetAnimation)